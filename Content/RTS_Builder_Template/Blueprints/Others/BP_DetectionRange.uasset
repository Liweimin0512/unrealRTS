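; Detection sphere actor that trails a BP_MasterUnit and auto-acquires enemies for it in the RTS template.
; OnSpawned sizes the sphere, registers itself on the unit and starts a looping timer that snaps it to the unit, destroying itself once that is gone.
; CheckOverlapping, not called here, sends an idle, damage-capable unit to attack the first hostile overlap: player versus AI, or AI of differing teams.
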(event Custom|On%20Spawned
  (params (Follow%20Actor :type Actor%20Object%20Reference) (Detection%20Zone%20Size :type Float%20%28single-precision%29))
  (Utilities|IsValid Follow%20Actor
    (:Is%20Valid
      (Variables|Default|SetFollowing%20Actor Follow%20Actor)
      (Components|Sphere|SetSphereRadius (Variables|Default|GetDetection%20Sphere) Detection%20Zone%20Size true)
      (bind _asbp_master_unit (Utilities|Casting|CastToBP_MasterUnit (Variables|Default|GetFollowing%20Actor))
        (:then
          (Variables|Default|SetFollowing%20Unit _asbp_master_unit)
          (Utilities|Time|SetTimerbyEvent (delegate Custom|Follow%20Actor) 0.25 true)
          (Variables|/Game/RTS_Builder_Template/Blueprints/UnitActors/BP_MasterUnit.BP_MasterUnit_C|SetDetection%20Range (Variables|Default|GetFollowing%20Unit) self))
        (:CastFailed
          (Transformation|SetActorLocationAndRotation (Transformation|GetActorLocation (Variables|Default|GetFollowing%20Actor)) "0, 0, 0"))))
    (:Is%20Not%20Valid
      (Actor|DestroyActor))))

(event Custom|Follow%20Actor
  (Utilities|IsValid (Variables|Default|GetFollowing%20Actor)
    (:Is%20Valid
      (Transformation|SetActorLocationAndRotation (Transformation|GetActorLocation (Variables|Default|GetFollowing%20Actor)) "0, 0, 0"))
    (:Is%20Not%20Valid
      (Actor|DestroyActor))))

(fn ConstructionScript)

(fn CheckOverlapping
  (bind _following_unit (Variables|Default|GetFollowing%20Unit))
  (Utilities|IsValid _following_unit
    (:Is%20Valid
      (if (not (Variables|/Game/RTS_Builder_Template/Blueprints/UnitActors/BP_MasterUnit.BP_MasterUnit_C|GetPlay%20Order _following_unit))
        (if (not (Variables|/Game/RTS_Builder_Template/Blueprints/UnitActors/BP_MasterUnit.BP_MasterUnit_C|GetIs%20Attacking _following_unit))
          (bind _array_element (Utilities|Array|ForEachLoopwithBreak (Collision|GetOverlappingActors (Variables|Default|GetDetection%20Sphere) "/Game/RTS_Builder_Template/Blueprints/UnitActors/BP_MasterUnit.BP_MasterUnit_C" :!class /Script/Engine.PrimitiveComponent) :!label _label)
            (:LoopBody
              (bind _asbp_master_unit (Utilities|Casting|CastToBP_MasterUnit _array_element))
              (LocalVariables|SetOverlapping%20Unit _asbp_master_unit)
              (if (> (Variables|/Game/RTS_Builder_Template/Blueprints/UnitActors/BP_MasterUnit.BP_MasterUnit_C|GetDamage (Variables|Default|GetFollowing%20Unit)) 0.0)
                (if (Variables|/Game/RTS_Builder_Template/Blueprints/UnitActors/BP_MasterUnit.BP_MasterUnit_C|GetAI%20Controlled (LocalVariables|GetOverlapping%20Unit))
                  (if (Variables|/Game/RTS_Builder_Template/Blueprints/UnitActors/BP_MasterUnit.BP_MasterUnit_C|GetAI%20Controlled (Variables|Default|GetFollowing%20Unit))
                    (if (not (Utilities|Enum|Equal(Enum) (Variables|/Game/RTS_Builder_Template/Blueprints/UnitActors/BP_MasterUnit.BP_MasterUnit_C|GetTeam (LocalVariables|GetOverlapping%20Unit)) (Variables|/Game/RTS_Builder_Template/Blueprints/UnitActors/BP_MasterUnit.BP_MasterUnit_C|GetTeam (Variables|Default|GetFollowing%20Unit))))
                      (Default|MoveUnitto (Variables|Default|GetFollowing%20Unit) "0, 0, 0" "0, 0, 0" false (LocalVariables|GetOverlapping%20Unit) :!label _label_2)
                      (Default|BeginAttack (Variables|Default|GetFollowing%20Unit) (LocalVariables|GetOverlapping%20Unit) false)
                      (goto _label Break))
                    (else
                      (goto _label_2)))
                  (elif (Variables|/Game/RTS_Builder_Template/Blueprints/UnitActors/BP_MasterUnit.BP_MasterUnit_C|GetAI%20Controlled (Variables|Default|GetFollowing%20Unit))
                    (goto _label_2)))))))))
    (:Is%20Not%20Valid
      (Actor|DestroyActor))))
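; Base resource actor for the RTS builder template, holding a depletable amount of a resource.
; The construction script fills it to full, optionally randomizes the mesh's per-axis scale and yaw for variety, and sizes the selection ring from the mesh scale plus an offset.
; DeductResources subtracts a requested amount, returning true while some remains, or zeroing the total and returning false when the request meets or exceeds it.
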(fn `Deduct Resources`
  (params (`Deduct Amount` :type Integer))
  (returns (`Resources Remaining` :type Boolean))
  ;[1 1 1] Deduct the resources from this resource
  (if (> (`self.Current Resources`) `Deduct Amount`)
    (set `self.Current Resources` (- (`self.Current Resources`) `Deduct Amount`))
    (return true)
    (else
      (set `self.Current Resources` 0)
      (return false))))

(fn `UserConstructionScript`
  (bind _returnvalue (`KismetMathLibrary.RandomFloatInRange` (`self.Min Mesh Size`) (`self.Max Mesh Size`)))
  ;[1 1 1] Set Resources
  (set `self.Current Resources` (`self.Full Resources`))
  ;[1 1 1] If True Use Random Size
  (if (`self.Use Random Size`)
    ;[1 1 1] Set 3D World Size
    (`SceneComponent.SetWorldScale3D` (`self.ResourceMesh`) (`KismetMathLibrary.MakeVector` _returnvalue _returnvalue _returnvalue)))
  ;[1 1 1] If True Use Random Rotation
  (if (`self.Use Random Rotation`)
    ;[1 1 1] Set Random Rotation
    (`SceneComponent.K2_SetWorldRotation` (`self.ResourceMesh`) (`KismetMathLibrary.MakeRotator` 0.0 0.0 (`KismetMathLibrary.RandomFloatInRange` 0.0 365.0)) false false))
  ;[1 1 1] Set the selection ring size
  (`SceneComponent.SetWorldScale3D` (`self.SelectionRing`) (+ (`SceneComponent.K2_GetComponentScale` (`self.ResourceMesh`)) (1.5 1.5 1.5))))